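; DVA avalanche-transceiver display: a grabbable device that guides the player to the first Victime actor found at BeginPlay.
; A distance-scaled Delay on Tick paces readout and beeps, which quicken and rise in pitch when closer; the readout hides beyond 30 m and gains decimals under 5 m.
; An arrow pitches toward the victim every frame.
; Custom events handle attach/detach and input; E toggles an animated button that hides readout and arrow.
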(event `self.ReceiveBeginPlay`
  ;[1 0.8369 0.3533] position victime
  (bind _outactors (`GameplayStatics.GetAllActorsOfClass` "/Game/Xavier/blueprint/victime/Victime.Victime_C")))

(event `self.Sphere.OnComponentEndOverlap`
  (params (OverlappedComponent :type "PrimitiveComponent Object Reference") (OtherActor :type "Actor Object Reference") (OtherComp :type "PrimitiveComponent Object Reference") (OtherBodyIndex :type Integer))
  ;[0.5697 0.4631 1] position DVA
)

(event `self.Sphere.OnComponentBeginOverlap`
  (params (OverlappedComponent :type "PrimitiveComponent Object Reference") (OtherActor :type "Actor Object Reference") (OtherComp :type "PrimitiveComponent Object Reference") (OtherBodyIndex :type Integer) (bFromSweep :type Boolean) (SweepResult :type "HitResult Structure (by ref)"))
  ;[0.5697 0.4631 1] position DVA
)

(event `self.ReceiveTick`
  (params (DeltaSeconds :type "Float (single-precision)"))
  (bind _audio (`self.Audio`))
  (bind _rotationfleche (`self.RotationFleche`))
  ;[1 0.1369 0.09913] Depart
  (`|ExecutionSequence`
    (:`then_0`
      (bind _position_victime (`/Game/Xavier/blueprint/victime/Victime.Position Victime` (`|GetArrayItem` (stale `self.ReceiveBeginPlay` _outactors))))
      (bind _returnvalue (/ (`KismetMathLibrary.Conv_IntToDouble` (`KismetMathLibrary.FTrunc` (`KismetMathLibrary.VSize` (- (`self.position acteur`) _position_victime)))) 100.0))
      (`KismetSystemLibrary.Delay` (`KismetMathLibrary.MapRangeClamped` _returnvalue 0.0 30.0 0.05 1.5))
      (`|ExecutionSequence`
        (:`then_0`
          ;[1 0.8761 0.2622] position acteur
          (set `self.position acteur` (`SceneComponent.K2_GetComponentLocation` (`self.Sphere`))))
        (:`then_2`
          (if (>= _returnvalue 5.0)
            ;[0.4169 1 0.4451] affichage distance
            (`TextRenderComponent.K2_SetText` (`self.distance`) (`KismetTextLibrary.Conv_IntToText` (`KismetMathLibrary.Round` _returnvalue)))
            (else
              ;[0.3613 1 0.3863] afficher distance precise
              (`TextRenderComponent.K2_SetText` (`self.distance`) (`KismetTextLibrary.Conv_DoubleToText` _returnvalue "HalfToEven"))))
          ;[0.4343 1 0.4349] rendre visible distance
          (`SceneComponent.SetVisibility` (`self.distance`) (<= _returnvalue 30.0) false))
        (:`then_3`
          ;[1 0 0.7813] song distance
          (`AudioComponent.SetPitchMultiplier` _audio (`KismetMathLibrary.MapRangeClamped` _returnvalue 0.0 30.0 2.0 1.2))
          (`AudioComponent.Play` _audio 0.0))))
    (:`then_1`
      (bind (_returnvalue_roll _returnvalue_pitch) (`KismetMathLibrary.BreakRotator` (`KismetMathLibrary.FindLookAtRotation` (`SceneComponent.K2_GetComponentLocation` _rotationfleche) _position_victime)))
      ;[0.2713 1 0.9303] Ajuster en fonction des axes nécéssaires
      (`SceneComponent.K2_SetRelativeRotation` _rotationfleche (`KismetMathLibrary.MakeRotator` 0.0 _returnvalue_pitch) false false))))

(event `CustomEvent_1`
  (params (AttachTo :type "SceneComponent Object Reference"))
  ;[0.4429 0.359 1] attrper DVA
  (`PrimitiveComponent.SetSimulatePhysics` (`self.Sphere`) false)
  (`SceneComponent.K2_AttachToComponent` (`self.K2_GetRootComponent`) AttachTo "None" "KeepWorld" "KeepWorld" "KeepWorld" false))

(event `CustomEvent_2`
  ;[0.4429 0.359 1] attrper DVA
  (`PrimitiveComponent.SetSimulatePhysics` (`self.Sphere`) true)
  (`self.K2_DetachFromActor` "KeepWorld" "KeepWorld" "KeepWorld"))

(event `Key|E` :consume false
  (params (Key :type "Key Structure"))
  ;[1 0.2731 0.3229] bouton
  (:`Pressed`
    (`/Engine/EditorBlueprintResources/StandardMacros.FlipFlop`
      (:`A`
        (`GameplayStatics.PlaySound2D` null 1.0 1.0 0.0 null null)
        (bind (_direction _newtrack_0) (`Timeline|Timeline_0` :!label _label)
          (:`Update`
            (`SceneComponent.K2_SetRelativeLocation` (`self.boutton`) (`KismetMathLibrary.MakeVector` 0.0 _newtrack_0) false false)
            (`|ExecutionSequence`
              (:`then_0`
                (`SceneComponent.SetVisibility` (`self.distance`) false false))
              (:`then_1`
                (`SceneComponent.SetVisibility` (`self.fleche`) false false))))))
      (:`B`
        (`GameplayStatics.PlaySound2D` null 1.0 0.5 0.0 null null)
        (goto _label :!via `Reverse`)))))

(event `CustomEvent`
  ;[1 1 1] blowprint qui ecoute
  (`self.EnableInput` (`GameplayStatics.GetPlayerController` 0)))

(fn `Compass`)

(fn `UserConstructionScript`)