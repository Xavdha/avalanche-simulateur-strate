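; Countdown timer Blueprint with a TextRender display that ends play when time runs out.
; A Delay on Tick acts as a one-second clock, decrementing Secondes and rolling it over into Minutes.
; When both reach zero, it prints that the victim is probably dead and pauses the game.
; A parallel Sequence branch refreshes the text every tick from an int-to-text conversion, with no input variable shown.
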(event `self.ReceiveTick`
  (params (DeltaSeconds :type "Float (single-precision)"))
  (`|ExecutionSequence`
    (:`then_0`
      (`KismetSystemLibrary.Delay` 1.0)
      (set `self.secondes` (- (`self.secondes`) 1))
      (if (< (`self.secondes`) 0)
        (set `self.minutes` (- (`self.minutes`) 1))
        (set `self.secondes` 59))
      (if (== (`self.secondes`) 0)
        (if (== (`self.minutes`) 0)
          (`KismetSystemLibrary.PrintString` "THE VICTIME IS PROBABLY DEAD")
          (`GameplayStatics.SetGamePaused` true))))
    (:`then_1`
      (`TextRenderComponent.K2_SetText` (`self.TextRender`) (`KismetTextLibrary.Conv_IntToText` 0)))))

(fn `UserConstructionScript`)